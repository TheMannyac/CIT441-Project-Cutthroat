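; Stationary enemy sentry that tracks a target with its turret and fires projectiles on a looping timer.
; BeginPlay targets the player pawn and starts the timer only if no target is preset; the timer pauses once the target is invalid.
; Tick aims the Sentry component using hand-built Atan2 yaw and pitch.
; ShootAtTarget spawns the projectile with sound, but assigns the bullet's target only on the cast's failure branch.
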(event `self.ReceiveBeginPlay`
  ;[1 1 1] Set Target On Creation
  (`/Engine/EditorBlueprintResources/StandardMacros.IsValid` (`self.TargetActor`)
    (:`Is Not Valid`
      (bind _output_get (set `self.TargetActor` (`GameplayStatics.GetPlayerPawn` 0)))
      (`/Engine/EditorBlueprintResources/StandardMacros.IsValid` _output_get
        (:`Is Valid`
          (bind _returnvalue (`KismetSystemLibrary.K2_SetTimerDelegate` (delegate `On Shoot`) (`self.Attack interval`) true (`self.Initial Start Delay`)))
          (set `self.Attack Timer Handle` _returnvalue))))))

(event `On Shoot`
  ;[1 1 1] Attack
  (`self.ShootAtTarget`)
  (`/Engine/EditorBlueprintResources/StandardMacros.IsValid` (`self.TargetActor`)
    (:`Is Not Valid`
      (`KismetSystemLibrary.K2_PauseTimerHandle` (`self.Attack Timer Handle`)))))

(event `self.ReceiveTick`
  (params (DeltaSeconds :type "Float (single-precision)"))
  (bind _x (.x (`self.DirectionToTarget`)))
  (bind _y (.y (`self.DirectionToTarget`)))
  (bind _returnvalue (- (`self.K2_GetActorLocation` (`self.TargetActor`)) (`SceneComponent.K2_GetComponentLocation` (`self.Shoot point`))))
  (`|ExecutionSequence`
    (:`then_0`
      ;[1 1 1] Get Direciton and Distance from target
      (`/Engine/EditorBlueprintResources/StandardMacros.IsValid` (`self.TargetActor`)
        (:`Is Valid`
          (set `self.DirectionToTarget` (`KismetMathLibrary.Normal` _returnvalue))
          (set `self.DistanceToTarget` (`KismetMathLibrary.VSize` _returnvalue)))))
    (:`then_1`
      ;[1 1 1] This is the trig involved in the above nodes like 'Make Rot from X' (minus some error handling/validation)
      ; 3D Rotation is broken into 2 2D Rotations, 1 around the up axis, then 1 around the actor's right vector so it looks up or down.
      (`SceneComponent.K2_SetRelativeRotation` (`self.sentry`) (`KismetMathLibrary.ComposeRotators` (`KismetMathLibrary.MakeRotator` 0.0 (`KismetMathLibrary.DegAtan2` (.z (`self.DirectionToTarget`)) (`KismetMathLibrary.Sqrt` (+ (* _x _x) (* _y _y))))) (`KismetMathLibrary.MakeRotator` 0.0 0.0 (+ (`KismetMathLibrary.DegAtan2` _y _x) (`self.yaw offset`)))) false false))
    (:`then_2`)))

(fn `ShootAtTarget`
  (bind (_returnvalue_location _returnvalue_rotation) (`KismetMathLibrary.BreakTransform` (`SceneComponent.K2_GetComponentToWorld` (`self.Shoot point`))))
  (bind _returnvalue (`|SpawnActorFromClass` (`self.projectile`) (`SceneComponent.K2_GetComponentToWorld` (`self.Shoot point`)) "AlwaysSpawn" "OverrideRootScale" self self))
  (bind _asbp_bullet (cast `/Game/Blueprints/Combat/Projectiles/bp_bullet` _returnvalue)
    (:`then`
      _)
    (:`CastFailed`
      (set `/Game/Blueprints/Combat/Projectiles/bp_bullet.target actor` (`self.TargetActor`) _asbp_bullet)))
  (`GameplayStatics.PlaySoundAtLocation` "/Game/ImportedAssets/Audio/laserLarge_001.laserLarge_001" _returnvalue_location _returnvalue_rotation 0.6 1.0 0.0 null null self)
  (`KismetSystemLibrary.PrintString` "shoot"))

(fn `UserConstructionScript`)