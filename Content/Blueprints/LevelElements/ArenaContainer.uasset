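; ArenaContainer is a level element that groups an arena's keys and gate so the arena can be reset.
; One second after BeginPlay it uses actor overlaps to store each Arena_key's location and the first ArenaGate found, printing debug messages.
; ResetArena calls Open(false) on that gate and spawns a new key at every saved location, without removing existing keys.
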(event `self.ReceiveBeginPlay`
  (bind _output (`|GetArrayItem` (`self.GetOverlappingActors` "/Game/Blueprints/LevelElements/ArenaGate.ArenaGate_C")))
  ;[1 1 1] Get all keys and their locations
  (`KismetSystemLibrary.Delay` 1.0)
  (for _array_element (`self.GetOverlappingActors` "/Game/Blueprints/LevelElements/arena_key.arena_key_C")
    (`KismetArrayLibrary.Array_Add` (`self.Keys`) (`self.K2_GetActorLocation` _array_element))
    (`KismetSystemLibrary.PrintString` "triggered" true true (struct :`R` 0.981924 :`B` 1.0 :`A` 1.0)))
  ;[1 1 1] Get arena gate
  (bind _asarena_gate (cast `/Game/Blueprints/LevelElements/ArenaGate` _output))
  (set `self.GateToOpen` _asarena_gate)
  (`KismetSystemLibrary.PrintString` "Arena gate set")
  (`KismetSystemLibrary.PrintString` (`KismetSystemLibrary.GetDisplayName` _output))
  (`KismetSystemLibrary.PrintString` "Array length: ")
  (`KismetSystemLibrary.PrintString` (`KismetStringLibrary.Conv_IntToString` (`KismetArrayLibrary.Array_Length` (`self.Keys`))) true true (struct :`R` 1.0 :`G` 0.109007 :`A` 1.0) 5.0))

(fn `ResetArena`
  (`/Game/Blueprints/LevelElements/ArenaGate.Open` (`self.GateToOpen`) false)
  (for _array_element (`self.Keys`)
    (`|SpawnActorFromClass` "/Game/Blueprints/LevelElements/arena_key.arena_key_C" (`KismetMathLibrary.Conv_VectorToTransform` _array_element) "AdjustIfPossibleButAlwaysSpawn" "OverrideRootScale" null null)))

(fn `UserConstructionScript`)