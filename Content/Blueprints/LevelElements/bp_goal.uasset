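; Goal pickup actor for a level that shows a win screen when the player reaches it.
; Tick bobs it on a sine wave around its starting location and spins it in yaw, both driven by time since creation.
; Overlapping its sphere with an actor of exactly the Bp_player class creates the win widget and adds it to the viewport, guarded so only one is shown.
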(event `self.ReceiveBeginPlay`
  (set `self.starting location` (`self.K2_GetActorLocation`)))

(event `self.ReceiveTick`
  (params (DeltaSeconds :type "Float (single-precision)"))
  (bind (_starting_location_x _starting_location_y _starting_location_z) (`KismetMathLibrary.BreakVector` (`self.starting location`)))
  (`self.K2_SetActorLocationAndRotation` (`KismetMathLibrary.MakeVector` _starting_location_x _starting_location_y (+ _starting_location_z (* (`self.float offset`) (`KismetMathLibrary.Sin` (* (`self.GetGameTimeSinceCreation`) 0.7))))) (`KismetMathLibrary.MakeRotator` 0.0 0.0 (mod (* (`self.GetGameTimeSinceCreation`) (`self.rotation rate`)) 360.0))))

(event `self.Sphere.OnComponentBeginOverlap`
  (params (OverlappedComponent :type "PrimitiveComponent Object Reference") (OtherActor :type "Actor Object Reference") (OtherComp :type "PrimitiveComponent Object Reference") (OtherBodyIndex :type Integer) (bFromSweep :type Boolean) (SweepResult :type "HitResult Structure (by ref)"))
  (if (and (== (`GameplayStatics.GetObjectClass` OtherActor) "/Game/Blueprints/Player/bp_player.bp_player_C") (not (`KismetSystemLibrary.IsValid` (`self.winScreen`))))
    (bind _returnvalue (`|CreateWidget` "/Game/Blueprints/UI/winScreen.winScreen_C" (`GameplayStatics.GetPlayerController` 0)))
    (set `self.winScreen` _returnvalue)
    (`UserWidget.AddToViewport` _returnvalue 0)
    (if true
      _)))

(fn `UserConstructionScript`)