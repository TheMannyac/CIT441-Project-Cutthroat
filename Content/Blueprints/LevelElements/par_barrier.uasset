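; Parent-style breakable barrier level element that shatters with a glass sound and respawns after a delay.
; Breaking hides the barrier component, disables its collision and starts a one-shot respawn timer.
; Respawn restores visibility and collision with a sound, and both transitions update IsBarrierActive, call broken/respawn notifications and print debug text.
; The break trigger is not in this graph; OnBarrierBroken receives the hit that positions the sound.
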(event `On Barrier Broken`
  (params (`Breaking Hit` :type "HitResult Structure"))
  (bind _barrier (`self.barrier`))
  ;[1 1 1] Barrier Broken
  (`PrimitiveComponent.SetCollisionEnabled` _barrier "NoCollision")
  (`SceneComponent.SetVisibility` _barrier false true)
  (`GameplayStatics.PlaySoundAtLocation` "/Game/ImportedAssets/Audio/glassBreaking.glassBreaking" (`.Location` (`GameplayStatics.BreakHitResult` `Breaking Hit`)) (struct) 1.0 1.0 0.0 null null null)
  (bind _returnvalue (`KismetSystemLibrary.K2_SetTimerDelegate` (delegate `On Respawn`) (`self.respawnDelay`)))
  (set `self.Respawn Timer` _returnvalue)
  (set `self.isBarrierActive` false)
  (`self.Barrier Broken`)
  (`KismetSystemLibrary.PrintString` "Barrier Broken" true true (struct :`R` 0.190644 :`G` 0.215587 :`B` 1.0 :`A` 1.0)))

(event `On Respawn`
  (bind _barrier (`self.barrier`))
  ;[1 1 1] Barrier REspawn
  (`KismetSystemLibrary.K2_ClearAndInvalidateTimerHandle` (`self.Respawn Timer`))
  ;;[1 1 1] Re-enable Barrier
  (`PrimitiveComponent.SetCollisionEnabled` _barrier "QueryAndPhysics")
  (`SceneComponent.SetVisibility` _barrier true true)
  (`GameplayStatics.PlaySoundAtLocation` "/Game/ImportedAssets/Audio/Celeste/powerupRespawn.powerupRespawn" (`self.K2_GetActorLocation`) (struct) 1.0 1.0 0.0 null null self)
  (set `self.isBarrierActive` true)
  (`self.Barrier Respawn`)
  (`KismetSystemLibrary.PrintString` "Barrier Respawned"))

(fn `UserConstructionScript`)