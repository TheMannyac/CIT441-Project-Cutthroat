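; A drawbridge level element that raises and lowers by pitching its static mesh when activated.
; Each Activate flips an up/down flag and plays or reverses a timeline, whose percent interpolates the relative pitch between flat and a configurable rotation amount.
; Indicate and UnIndicate toggle custom depth rendering on the mesh to mark the bridge visually.
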(event `/Game/Blueprints/Interfaces/Interactable.Activate`
  (bind _isgoingup (`self.isGoingUp`))
  (set `self.isGoingUp` (not _isgoingup))
  (if _isgoingup
    (bind (_direction _percent) (`Timeline|RotateBridge` :!label _label)
      (:`Update`
        (`SceneComponent.K2_SetRelativeRotation` (`self.StaticMesh`) (`KismetMathLibrary.MakeRotator` 0.0 (`KismetMathLibrary.Lerp` 0.0 (`self.RotateAmount`) _percent)) false false)))
    (else
      (goto _label :!via `Reverse`))))

(event `/Game/Blueprints/Interfaces/Interactable.Indicate`
  (`PrimitiveComponent.SetRenderCustomDepth` (`self.StaticMesh`) true))

(event `/Game/Blueprints/Interfaces/Interactable.UnIndicate`
  (`PrimitiveComponent.SetRenderCustomDepth` (`self.StaticMesh`) false))

(fn `UserConstructionScript`)