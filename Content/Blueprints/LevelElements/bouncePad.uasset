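; Bounce pad level element that launches the player when a Bouncable actor hits its Pad component.
; Only the Fixed launch type is wired: it launches bp_player along the pad's up vector with a set velocity and plays a bounce sound.
; The construction script colours the pad by LaunchType (Fixed, Relative, Scripted) and matches Bottom's material to Rim's.
; Relative launch, older code and rotation-math experiments remain disconnected.
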(event `self.pad.OnComponentHit`
  (params (HitComponent :type "PrimitiveComponent Object Reference") (OtherActor :type "Actor Object Reference") (OtherComp :type "PrimitiveComponent Object Reference") (NormalImpulse :type "Vector Structure") (Hit :type "HitResult Structure (by ref)"))
  (bind (_returnvalue_location _returnvalue_rotation) (`KismetMathLibrary.BreakTransform` (`self.GetTransform`)))
  (bind _asbouncable (cast `/Game/Bouncable` OtherActor))
  (switch `/Game/Blueprints/LevelElements/eJumpPadLaunchType` (`self.Launch Type`)
    (:`NewEnumerator1`
      ;[0.3042 1 0] Fixed
      (bind _asbp_player (cast `/Game/Blueprints/Player/bp_player` _asbouncable))
      (`Character.LaunchCharacter` _asbp_player (* (`SceneComponent.GetUpVector` (`self.pad`)) (`self.Fixed Launch Velocity`)) (`self.fixedXYOverride`) true)
      (`GameplayStatics.PlaySoundAtLocation` "/Game/ImportedAssets/Audio/bounce.bounce" _returnvalue_location _returnvalue_rotation 1.0 1.0 0.0 null null null)
      (`KismetSystemLibrary.PrintString` "Fixed Launch" true true (struct :`R` 1.0 :`G` 0.685831 :`B` 0.024942 :`A` 1.0)))))

(fn `UserConstructionScript`
  (bind _pad (`self.pad`))
  (`|ExecutionSequence`
    (:`then_0`
      (switch `/Game/Blueprints/LevelElements/eJumpPadLaunchType` (`self.Launch Type`)
        (:`NewEnumerator1`
          ;[1 1 1] Launch ovverides the affectd pawn's velocity and direction for consistency, but does disable affected pawn's ability to move.
          (`PrimitiveComponent.SetMaterial` _pad 0 "/Game/ImportedAssets/MundellsStarterContent/Materials/Orange.Orange"))
        (:`NewEnumerator0`
          ;[1 1 1] Direction & Velocity of launch relative to that of the affected pawn before the launch. Functions like  a trampoline.
          (`PrimitiveComponent.SetMaterial` _pad 0 "/Game/ImportedAssets/MundellsStarterContent/Materials/ForestGreen.ForestGreen"))
        (:`NewEnumerator2`
          ;[1 1 1] Launch Picks a place on the map and lerps them to that location over a fixed period of time, and temporarily disable's the pawn's directional controller. Good for Sonic-esque scripted platforming sequences.
          (`PrimitiveComponent.SetMaterial` _pad 0 "/Game/ImportedAssets/MundellsStarterContent/Materials/Red.Red"))))
    (:`then_1`
      (`PrimitiveComponent.SetMaterial` (`self.bottom`) 0 (`|GetArrayItem` (`MeshComponent.GetMaterials` (`self.rim`)))))))