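; Interactable actor that slides between two offset positions when activated, with a custom-depth highlight while it is indicated and interactable.
; Activate disables interaction and drives a timeline that lerps the actor's location, with play rate inverted from PlayRate.
; It either returns itself after a rest delay or alternates direction per activation, with optional cooldown.
; The construction script previews the mesh along the path and configures scale and the interaction sphere.
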(event `/Game/Blueprints/Interfaces/Interactable.Indicate`
  ;[1 1 1] Turn highlight on (fires once)
  (`PrimitiveComponent.SetRenderCustomDepth` (`self.Mesh`) (`self.Interactable`)))

(event `/Game/Blueprints/Interfaces/Interactable.UnIndicate`
  ;[1 1 1] Turn highlight off (fires once)
  (`PrimitiveComponent.SetRenderCustomDepth` (`self.Mesh`) false))

(event `/Game/Blueprints/Interfaces/Interactable.Activate`
  (bind _isgoingup (`self.isGoingUp`))
  ;[1 1 1] Disable interaction while moving
  (if (`self.Interactable`)
    (set `self.Interactable` false)
    (`PrimitiveComponent.SetRenderCustomDepth` (`self.Mesh`) false)
    ;[1 1 1] Translate along path
    (if (`self.Resets Itself`)
      (bind (_direction _percent) (`Timeline|Translate` :!label _label)
        (:`Update`
          (bind _output_get (set `self.PercentOnPath` _percent))
          (`self.K2_SetActorLocation` (`KismetMathLibrary.VLerp` (`self.StartWorldLocation`) (`self.EndWorldLocation`) _output_get)))
        (:`Finished`
          (if (`self.Resets Itself`)
            (if (`self.OnWayBack`)
              (`KismetSystemLibrary.RetriggerableDelay` (`self.InteractCooldown`))
              (set `self.Interactable` true)
              (set `self.OnWayBack` false)
              (else
                (`KismetSystemLibrary.RetriggerableDelay` (`self.RestTime`))
                (`self.Reverse`)
                (set `self.OnWayBack` true)))
            (else
              (set `self.Interactable` true)))))
      (else
        (if (> (`self.InteractCooldown`) 0.0)
          (`KismetSystemLibrary.RetriggerableDelay` (`self.InteractCooldown`))
          (set `self.Interactable` true))
        (set `self.isGoingUp` (not _isgoingup))
        (if _isgoingup
          (goto _label)
          (else
            (goto _label :!via `Reverse`)))))))

(event `Reverse`
  ;[1 1 1] Translate along path
  (goto _label :!via `Reverse`))

(event `self.ReceiveBeginPlay`
  (bind _returnvalue (`self.K2_GetActorLocation`))
  (`|ExecutionSequence`
    (:`then_0`
      ;[1 1 1] Set location variables
      (set `self.StartWorldLocation` (+ (`self.OriginalPosition`) _returnvalue))
      (set `self.EndWorldLocation` (+ (`self.PositionToMove`) _returnvalue)))
    (:`then_1`
      ;[1 1 1] Set play rate
      (`TimelineComponent.SetPlayRate` (`self.Translate`) (/ 1.0 (`self.Play rate`))))))

(fn `CanInteract`
  (returns (NewParam :type Boolean))
  (return (`self.Interactable`)))

(fn `UserConstructionScript`
  (`SceneComponent.K2_SetRelativeLocation` (`self.Mesh`) (`KismetMathLibrary.VLerp` (`self.OriginalPosition`) (`self.PositionToMove`) (`self.PathPercent`)) false false)
  (`SceneComponent.SetRelativeScale3D` (`self.Mesh`) (`self.Scale`))
  (`SphereComponent.SetSphereRadius` (`self.InteractionRadius`) (`self.InteractionBubbleRadius`) true)
  (`SceneComponent.K2_SetRelativeLocation` (`self.InteractionRadius`) (`self.InteractionBubbleLocation`) false false))