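; DashRing is a level element that launches bp_player along the ring's up vector when it overlaps the ring's sphere.
; It can first teleport the player to its center in Falling mode, then applies a fixed launch velocity and plays a sound pitched by launch strength.
; A DoOnce gate blocks retriggers while the ring and lights turn red, then resets after a short delay as they return to green.
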(event `self.Sphere.OnComponentBeginOverlap`
  (params (OverlappedComponent :type "PrimitiveComponent Object Reference") (OtherActor :type "Actor Object Reference") (OtherComp :type "PrimitiveComponent Object Reference") (OtherBodyIndex :type Integer) (bFromSweep :type Boolean) (SweepResult :type "HitResult Structure (by ref)"))
  (bind (_returnvalue_location _returnvalue_rotation) (`KismetMathLibrary.BreakTransform` (`self.GetTransform`)))
  (bind _linearcolor (make `LinearColor` 0.0 1.0))
  (bind _linearcolor_2 (make `LinearColor` 1.0))
  ;[1 1 1] Launch
  (`/Engine/EditorBlueprintResources/StandardMacros.DoOnce` false :!label _label
    (:`Completed`
      (bind _asbp_player (cast `/Game/Blueprints/Player/bp_player` OtherActor))
      (if (`self.MovePlayerToCenter`)
        (`self.K2_SetActorLocation` _asbp_player (`self.K2_GetActorLocation`) false false)
        (`CharacterMovementComponent.SetMovementMode` (`Character.CharacterMovement` _asbp_player) "MOVE_Falling" 0))
      (`Character.LaunchCharacter` _asbp_player (* (`SceneComponent.GetUpVector` (`self.Ring`)) (`self.FixedLaunchVelocity`)) (`self.fixedXYOverride`) true)
      (`GameplayStatics.PlaySoundAtLocation` "/Game/ImportedAssets/Audio/launchRing.launchRing" _returnvalue_location _returnvalue_rotation 1.0 (`KismetMathLibrary.FClamp` (/ (`self.FixedLaunchVelocity`) 3000.0) 1.0 1.2) 0.0 "/Game/Blueprints/DefaultAttenuation.DefaultAttenuation" null null)
      (`KismetSystemLibrary.PrintString` "Fixed Launch" false true (struct :`R` 1.0 :`G` 0.685831 :`B` 0.024942 :`A` 1.0))
      (`PrimitiveComponent.SetMaterial` (`self.Ring`) 0 "/Game/ImportedAssets/MundellsStarterContent/Materials/Red.Red")
      (`LightComponent.SetLightColor` (`self.PointLight`) _linearcolor_2 true)
      (`LightComponent.SetLightColor` (`self.PointLight1`) _linearcolor_2 true)
      (`KismetSystemLibrary.RetriggerableDelay` 1.0)
      (`PrimitiveComponent.SetMaterial` (`self.Ring`) 0 "/Game/ImportedAssets/MundellsStarterContent/Materials/Green.Green")
      (`LightComponent.SetLightColor` (`self.PointLight`) _linearcolor true)
      (`LightComponent.SetLightColor` (`self.PointLight1`) _linearcolor true)
      (`self.ResetRing`))))

(event `ResetRing`
  ;[1 1 1] Launch
  (goto _label :!via `Reset`))

(fn `UserConstructionScript`)