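; Spawner level element that marks a circular spawn area, with enemy spawning drafted but not wired to run.
; The construction script scales the SpawnRadius component from SpawnDiameter divided by 100.
; Disconnected EventGraph nodes would spawn an Enemy at a random flat offset around the actor, using SpawnDiameter as the maximum distance.
; A debug sphere draw is also left disconnected.
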(fn `UserConstructionScript`
  (`SceneComponent.SetWorldScale3D` (`self.Spawn Radius`) (`KismetMathLibrary.Conv_DoubleToVector` (/ (`self.spawnDiameter`) 100.0))))