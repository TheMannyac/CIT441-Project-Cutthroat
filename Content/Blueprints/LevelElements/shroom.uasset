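; Mushroom power-up that bobs and spins, and resets the player's midair moves on overlap to grant another jump.
; Collection hides it, disables collision and plays a sound whose pitch rises with the player's count of shrooms collected.
; It binds to that player's landed and destroyed events, either of which resets the count, unbinds, and re-enables the pickup with a sound after a short random delay.
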(event `self.ReceiveTick`
  (params (DeltaSeconds :type "Float (single-precision)"))
  (`|ExecutionSequence`
    (:`then_0`
      ;[1 1 1] Bobbing Animation
      (`SceneComponent.K2_SetRelativeLocation` (`self.StaticMesh`) (`KismetMathLibrary.MakeVector` 0.0 0.0 (* (`KismetMathLibrary.Sin` (* 5 (`KismetSystemLibrary.GetGameTimeInSeconds`))) 10.0)) false false))
    (:`then_1`
      (`SceneComponent.K2_AddRelativeRotation` (`self.StaticMesh`) (`KismetMathLibrary.MakeRotator` 0.0 0.0 (* (`self.rotation speed`) (`GameplayStatics.GetWorldDeltaSeconds`))) false false))))

(event `self.Sphere.OnComponentBeginOverlap`
  (params (OverlappedComponent :type "PrimitiveComponent Object Reference") (OtherActor :type "Actor Object Reference") (OtherComp :type "PrimitiveComponent Object Reference") (OtherBodyIndex :type Integer) (bFromSweep :type Boolean) (SweepResult :type "HitResult Structure (by ref)"))
  (bind _affected_player_object (`self.Affected player object`))
  (`|ExecutionSequence`
    (:`then_0`
      ;[1 1 1] Powerup Collected
      (bind _asbp_player (cast `/Game/Blueprints/Player/bp_player` OtherActor))
      ;;[1 1 1] Gives the player another jump
      (bind _output_get (set `self.Affected player object` _asbp_player))
      (`/Game/Blueprints/Player/bp_player.Reset Midair Moves` _output_get)
      (bind _shroomcollected (`/Game/Blueprints/Player/bp_player.shroomCollected` _output_get))
      (`self.Disable Powerup` _shroomcollected)
      (`/Engine/EditorBlueprintResources/StandardMacros.IncrementInt` _shroomcollected))
    (:`then_1`
      ;[1 1 1] Power Up re-enabled once player hits the ground or dies
      (`/Engine/EditorBlueprintResources/StandardMacros.IsValid` _affected_player_object
        (:`Is Valid`
          (add `/Game/Blueprints/Player/bp_player.On Player Landed` _affected_player_object (delegate `On Affected Player Lands`))
          (add `self.OnDestroyed` _affected_player_object (delegate `On Affected Player Dies`)))))))

(event `On Affected Player Lands`
  (params (hit :type "HitResult Structure"))
  (bind _affected_player_object (`self.Affected player object`))
  ;[1 1 1] Power Up re-enabled once player hits the ground or dies
  (`|ExecutionSequence` :!label _label
    (:`then_0`
      (`KismetSystemLibrary.Delay` (`KismetMathLibrary.RandomFloatInRange` 0.3 0.65))
      (`self.Re-Enable Powerup`))
    (:`then_1`
      ;;[1 1 1] Unbind events and clear affected player variable
      (set `/Game/Blueprints/Player/bp_player.shroomCollected` 0 _affected_player_object)
      (remove `/Game/Blueprints/Player/bp_player.On Player Landed` _affected_player_object (delegate `On Affected Player Lands`))
      (remove `self.OnDestroyed` _affected_player_object (delegate `On Affected Player Dies`))
      (set `self.Affected player object` (`self.NULL Object`)))))

(event `On Affected Player Dies`
  (params (DestroyedActor :type "Actor Object Reference"))
  ;[1 1 1] Power Up re-enabled once player hits the ground or dies
  (goto _label))

(fn `Disable Powerup`
  (params (`num collected` :type Integer))
  (`PrimitiveComponent.SetCollisionEnabled` (`self.Sphere`) "NoCollision")
  (`SceneComponent.SetVisibility` (`self.StaticMesh`) false false)
  (`GameplayStatics.PlaySound2D` "/Game/ImportedAssets/Audio/Celeste/usePowerup.usePowerup" 0.75 (+ (`self.base pitch`) (* `num collected` (`self.pitch increase`))) 0.0 null null))

(fn `Re-Enable Powerup`
  (`PrimitiveComponent.SetCollisionEnabled` (`self.Sphere`) "QueryAndPhysics")
  (`SceneComponent.SetVisibility` (`self.StaticMesh`) true false)
  (`GameplayStatics.PlaySound2D` "/Game/ImportedAssets/Audio/Celeste/powerupRespawn.powerupRespawn" 1.0 1.0 0.0 null null)
  (`KismetSystemLibrary.PrintString` "powerup reset"))

(fn `UserConstructionScript`)