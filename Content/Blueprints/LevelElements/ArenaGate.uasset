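; Arena gate level element with two pivots that swing open and closed.
; The Open function plays or reverses OpenTimeline according to its Opened flag.
; The timeline's track drives a rotator lerp that sets both pivots' relative rotation, with Pivot1's yaw modified separately from Pivot2's, apparently to mirror the swing.
; BeginPlay, overlap, Tick and the construction script are empty, so the gate relies on external calls to Open.
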(fn `Open`
  (params (Opened :type Boolean))
  (bind _opentimeline (`self.OpenTimeline`))
  (if Opened
    (`TimelineComponent.Play` _opentimeline)
    (else
      (`TimelineComponent.Reverse` _opentimeline))))

(fn `UserConstructionScript`)