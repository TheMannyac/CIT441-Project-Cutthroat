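; Force field barrier level element that drops when its linked switch button is pressed, opening the exit.
; On BeginPlay it binds SwitchON to the referenced switch's button-pressed event and stores its starting location, or prints an error if no switch is set.
; SwitchON disables the barrier's collision, hides it, plays a laser sound at the actor and prints a message that the player can leave.
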(event `self.ReceiveTick`
  (params (DeltaSeconds :type "Float (single-precision)")))

(event `Switch ON`
  (bind _barrier (`self.Barrier`))
  ;[1 1 1] If the button is pressed, then the force field is turned off
  (`PrimitiveComponent.SetCollisionEnabled` _barrier "NoCollision")
  (`SceneComponent.SetVisibility` _barrier false false)
  (`GameplayStatics.PlaySoundAtLocation` "/Game/ImportedAssets/MundellsStarterContent/Audio/Laser.Laser" (`self.K2_GetActorLocation`) (struct) 1.0 1.0 0.0 null null null)
  (`KismetSystemLibrary.PrintString` "ForceField Down! \nYou can now leave!" true true (struct :`G` 1.0 :`B` 0.154746 :`A` 1.0) 4.0))

(event `self.ReceiveBeginPlay`
  (bind _switchobjectreference (`self.switchObjectReference`))
  (`/Engine/EditorBlueprintResources/StandardMacros.IsValid` _switchobjectreference
    (:`Is Valid`
      (add `/Game/Blueprints/LevelElements/bp_button.Button Pressed` _switchobjectreference (delegate `Switch ON`))
      (set `self.starting location` (`self.K2_GetActorLocation`)))
    (:`Is Not Valid`
      ;[1 1 1] Display an Error Message
      (`KismetSystemLibrary.PrintString` (`KismetStringLibrary.Concat_StrStr` (`KismetSystemLibrary.GetObjectName` _switchobjectreference) " button object is not set!!!") true true (struct :`R` 1.0 :`G` 0.042889 :`A` 1.0)))))

(fn `UserConstructionScript`)