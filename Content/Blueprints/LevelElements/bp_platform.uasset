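; Moving platform level element intended to travel between its start position and an end point placed via a 3D widget.
; Start and end are converted to world positions at construction and BeginPlay, with a flag to preview the platform at the end.
; Tick lerps the actor between them by PathPercent.
; The direction branch is hardwired true, so the percent only decreases and the toggled Reverse is unused; a Speed-based offset is disconnected.
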(event `self.ReceiveBeginPlay`
  (`self.Set World Locations`))

(event `self.ReceiveTick`
  (params (DeltaSeconds :type "Float (single-precision)"))
  (`self.Move Platform Along Path`))

(fn `Move Platform Along Path`
  (bind _path_percent (`self.Path Percent`))
  (bind _path_percent_2 (`self.Path Percent`))
  (bind _returnvalue (* (`GameplayStatics.GetWorldDeltaSeconds`) 0.5))
  (if true
    (set `self.Path Percent` (- _path_percent _returnvalue))
    (else
      (set `self.Path Percent` (+ _path_percent _returnvalue))))
  (if (or (>= _path_percent_2 1.0) (<= _path_percent_2 0.0))
    (set `self.reverse` (not (`self.reverse`))))
  (`self.K2_SetActorLocation` (`KismetMathLibrary.VLerp` (`self.Start World Location`) (`self.End World Location`) (`self.Path Percent`))))

(fn `Set World Locations`
  (bind _returnvalue (`self.K2_GetActorLocation`))
  ;[1 1 1] When using show 3d widget, their postiions stay relative to the actor (even when it move). Must store the widget's world position on begin play by adding the widget location to the actor's world position
  ;;[1 1 1] Store begin world position
  (set `self.Start World Location` _returnvalue)
  ;;[1 1 1] Store End World locaiton
  (set `self.End World Location` (+ (`self.End World Location`) _returnvalue)))

(fn `UserConstructionScript`
  (`self.Set World Locations`)
  (if (`self.Show At End Location`)
    (`SceneComponent.K2_SetWorldLocation` (`self.Platform`) (`self.End World Location`) false false)
    (else
      (`SceneComponent.K2_SetWorldLocation` (`self.Platform`) (`self.Start World Location`) false false))))