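; Homing bullet projectile that calls death on a bp_player it overlaps, other than its owner, then destroys itself.
; On BeginPlay, if no target is set, it homes on the closest "Player"-tagged Pawn found within the initial ClosestDistance.
; A timer disables homing after DelockPercent of the lifespan, so the bullet stops tracking mid-flight.
; Tick spins the Orb component for a tumbling look.
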(event `Lock Off`
  (set `ProjectileMovementComponent.bIsHomingProjectile` false (`self.ProjectileMovement`)))

(event `self.ReceiveBeginPlay`
  ;[1 1 1] Setup Homing Targeting
  (`/Engine/EditorBlueprintResources/StandardMacros.IsValid` (`self.target actor`)
    (:`Is Not Valid`
      (`self.Lock On`)
      (`KismetSystemLibrary.K2_SetTimerDelegate` (delegate `Lock Off`) (* (`self.delockPercent`) (`self.GetLifeSpan`))))))

(event `Lock On`
  (bind _projectilemovement (`self.ProjectileMovement`))
  ;[1 1 1] Enable Homing
  (bind _homing_target (`self.Find Homing Target`))
  (set `ProjectileMovementComponent.HomingTargetComponent` _homing_target _projectilemovement)
  (set `ProjectileMovementComponent.bIsHomingProjectile` true _projectilemovement))

(event `self.Sphere.OnComponentBeginOverlap`
  (params (OverlappedComponent :type "PrimitiveComponent Object Reference") (OtherActor :type "Actor Object Reference") (OtherComp :type "PrimitiveComponent Object Reference") (OtherBodyIndex :type Integer) (bFromSweep :type Boolean) (SweepResult :type "HitResult Structure (by ref)"))
  ;[1 1 1] Collision
  (if (not (== OtherActor (`self.GetOwner`)))
    (bind _asbp_player (cast `/Game/Blueprints/Player/bp_player` OtherActor))
    (`/Game/Blueprints/Player/bp_player.Death` _asbp_player)
    (`self.K2_DestroyActor`)))

(event `self.ReceiveTick`
  (params (DeltaSeconds :type "Float (single-precision)"))
  ;[1 1 1] Projectile tumbling code
  (`SceneComponent.K2_AddLocalRotation` (`self.orb`) (* (`KismetMathLibrary.MakeRotFromYZ` (`self.GetActorRightVector`) (`self.GetActorForwardVector`)) (`self.RotSpeed`)) false false))

(fn `Find Homing Target`
  (returns (`homing target` :type "SceneComponent Object Reference"))
  (bind _outactors (`GameplayStatics.GetAllActorsOfClassWithTag` "/Script/Engine.Pawn" "Player"))
  (for _array_element _outactors
    (bind _returnvalue (`KismetMathLibrary.VSize` (- (`self.K2_GetActorLocation` _array_element) (`self.K2_GetActorLocation`))))
    (if (< _returnvalue (`self.Closest Distance`))
      (set `self.Closest Distance` _returnvalue)
      (set `self.target actor` _array_element)))
  (return (`self.GetComponentByClass` (`self.target actor`) "/Script/Engine.SceneComponent")))

(fn `UserConstructionScript`)