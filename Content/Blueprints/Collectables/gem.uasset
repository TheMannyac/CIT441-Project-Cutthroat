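; Collectable gem Blueprint that comes in five color variants, from Green to Gold, each with its own value.
; The Construction Script switches on GemVariant to set the static mesh material and the matching Value, so each placed gem is configured by that one variable.
; OnPickup only calls the parent implementation, leaving collection behavior to the parent class, and the event graph holds no active logic.
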(fn `On Pickup`
  (params (Collector :type "Actor Object Reference"))
  (`parent.On Pickup` Collector))

(fn `UserConstructionScript`
  (`parent.UserConstructionScript`)
  (switch `/Game/Blueprints/Enums/GemsTypes` (`self.gem Variant`)
    (:`NewEnumerator1`
      ;[1 1 1] Green Gem
      (`PrimitiveComponent.SetMaterial` (`self.StaticMesh`) 0 "/Game/Materials/gemGreen.gemGreen")
      (set `self.value` 1))
    (:`NewEnumerator2`
      ;[1 1 1] Blue Gem
      (`PrimitiveComponent.SetMaterial` (`self.StaticMesh`) 0 "/Game/Materials/gemBlue.gemBlue")
      (set `self.value` 5))
    (:`NewEnumerator0`
      ;[1 1 1] Red Gem
      (`PrimitiveComponent.SetMaterial` (`self.StaticMesh`) 0 "/Game/Materials/redGem.redGem")
      (set `self.value` 10))
    (:`NewEnumerator4`
      ;[1 1 1] Silver Gem
      (`PrimitiveComponent.SetMaterial` (`self.StaticMesh`) 0 "/Game/ImportedAssets/MundellsStarterContent/Materials/Metal.Metal")
      (set `self.value` 25))
    (:`NewEnumerator3`
      ;[1 1 1] Gold Gem
      (`PrimitiveComponent.SetMaterial` (`self.StaticMesh`) 0 "/Game/Materials/Battery.Battery")
      (set `self.value` 50))))