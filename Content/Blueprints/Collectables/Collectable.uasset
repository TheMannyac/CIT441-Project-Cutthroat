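; Base collectable pickup that spins its mesh and reacts when a Bp_player actor overlaps its sphere.
; The overlap fires the Collected dispatcher, whose bound handler calls OnPickup, a debug-print function, then plays a randomly pitched sound.
; Optional self-destruction runs only when a pickup sound is valid.
; BeginPlay picks a random rotation direction, but the Tick rotation does not use it.
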(event `self.Sphere.OnComponentBeginOverlap`
  (params (OverlappedComponent :type "PrimitiveComponent Object Reference") (OtherActor :type "Actor Object Reference") (OtherComp :type "PrimitiveComponent Object Reference") (OtherBodyIndex :type Integer) (bFromSweep :type Boolean) (SweepResult :type "HitResult Structure (by ref)"))
  ;[1 1 1] Check to see if it is collected. Only collected if touched by the player
  (if (== (`GameplayStatics.GetObjectClass` OtherActor) "/Game/Blueprints/Player/bp_player.bp_player_C")
    (`self.Collected` OtherActor)))

(event `On Collected`
  (params (collector :type "Actor Object Reference"))
  (bind _pickup_sound (`self.Pickup Sound`))
  ;[1 1 1] Destroy and play sound
  (`self.On Pickup` collector)
  (`/Engine/EditorBlueprintResources/StandardMacros.IsValid` _pickup_sound
    (:`Is Valid`
      (`GameplayStatics.PlaySound2D` _pickup_sound 0.8 (`KismetMathLibrary.RandomFloatInRange` 0.9 1.2) 0.0 null null)
      (if (`self.destroyOnCollect`)
        (`self.K2_DestroyActor`)))))

(event `self.ReceiveBeginPlay`
  ;[1 1 1] Set random rotation direction
  (`|ExecutionSequence`
    (:`then_0`
      (add `self.Collected` (delegate `On Collected`)))
    (:`then_1`
      (set `self.rot diration` (`KismetMathLibrary.SelectInt` 1 -1 (`KismetMathLibrary.RandomBool`))))))

(event `self.ReceiveTick`
  (params (DeltaSeconds :type "Float (single-precision)"))
  (bind _staticmesh (`self.StaticMesh`))
  ;[1 1 1] Rotation animation
  (`SceneComponent.K2_AddLocalRotation` _staticmesh (`KismetMathLibrary.Conv_VectorToRotator` (* (`SceneComponent.GetRightVector` _staticmesh) (* (`self.rotation speed`) (`GameplayStatics.GetWorldDeltaSeconds`)))) false false))

(fn `On Pickup`
  (params (Collector :type "Actor Object Reference"))
  (`KismetSystemLibrary.PrintString` "collected")
  (return))

(fn `UserConstructionScript`)