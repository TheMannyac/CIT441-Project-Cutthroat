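; Teleporter projectile that warps its owning character to where it lands on walkable floor.
; On hit, it compares the surface normal to the character's walkable floor Z, then swaps TeleNode to a lock material and starts a delay timer.
; When the timer fires, it moves the owner there, lifted by capsule half-height plus a buffer, snaps control yaw to the projectile's, plays a sound and destroys itself.
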(event `self.ReceiveTick`
  (params (DeltaSeconds :type "Float (single-precision)")))

(event `self.ReceiveBeginPlay`
  (`SceneComponent.K2_SetWorldRotation` :`self` (`self.TeleNode`)))

(event `self.ReceiveHit`
  (params (MyComp :type "PrimitiveComponent Object Reference") (Other :type "Actor Object Reference") (OtherComp :type "PrimitiveComponent Object Reference") (bSelfMoved :type Boolean) (HitLocation :type "Vector Structure") (HitNormal :type "Vector Structure") (NormalImpulse :type "Vector Structure") (Hit :type "HitResult Structure (by ref)"))
  ;[1 1 1] Initiate Teleport
  ;;[1 1 1] First checks if teleporter has hit the floor and not a wall
  (bind _ascharacter (cast `Character` (`self.GetOwner`)))
  (if (< (`CharacterMovementComponent.K2_GetWalkableFloorZ` (`Character.CharacterMovement` _ascharacter)) (.z HitNormal))
    (bind _returnvalue (`KismetSystemLibrary.K2_SetTimerDelegate` (delegate `Warp Player`) (`self.Teleport Delay`)))
    (set `self.warpTimerHandle` _returnvalue)
    (`PrimitiveComponent.SetMaterial` (`self.TeleNode`) 1 (`self.lockMaterial`))
    (`self.On Projectile Hit` 0.0 Hit)))

(event `self.ReceiveDestroyed`
  ;[1 1 1] Clear the Timer if the teleporter gets prematurely destroyed somehow.
  (`KismetSystemLibrary.K2_ClearAndInvalidateTimerHandle` (`self.warpTimerHandle`)))

(event `Warp Player`
  (bind _returnvalue (`self.GetOwner`))
  (bind _returnvalue_location (`KismetMathLibrary.BreakTransform` (`self.GetTransform`)))
  (bind (_ascharacter _bsuccess) (cast `Character` _returnvalue :!pure true))
  ;[1 1 1] Teleport
  (`/Engine/EditorBlueprintResources/StandardMacros.IsValid` _returnvalue
    (:`Is Valid`
      (`self.K2_SetActorLocation` _returnvalue (+ _returnvalue_location (`KismetMathLibrary.SelectVector` (`KismetMathLibrary.MakeVector` 0.0 0.0 (+ (`CapsuleComponent.GetScaledCapsuleHalfHeight` (`Character.CapsuleComponent` _ascharacter)) (`self.characterSpawnZBuffer`))) (0.0 0.0 0.0) _bsuccess)) false true)
      (bind _aspawn (cast `Pawn` _returnvalue)
        (:`then`
          (`self.Snap Player Camera` _aspawn))
        (:`CastFailed`
          _))
      (`GameplayStatics.PlaySoundAtLocation` "/Game/Audio/SFX/warp.warp" (`self.K2_GetActorLocation`) (struct) 1.0 1.0 0.0 null null null)
      (`self.K2_DestroyActor`)
      (`KismetSystemLibrary.PrintString` "Player teleported" true true (struct :`R` 1.0 :`G` 0.19938 :`A` 1.0)))))

(fn `Projectile Hit`
  (params (`Other Actor` :type "Actor Object Reference")))

(fn `Snap Player Camera`
  (params (`Owning Plawn` :type "Pawn Object Reference"))
  (bind (_returnvalue_roll _returnvalue_pitch _returnvalue_yaw) (`KismetMathLibrary.BreakRotator` (`self.K2_GetActorRotation`)))
  (bind _returnvalue (`Pawn.GetController` `Owning Plawn`))
  (bind (_returnvalue_roll_2 _returnvalue_pitch_2) (`KismetMathLibrary.BreakRotator` (`Controller.GetControlRotation` _returnvalue)))
  ;[1 1 1] Snap the Player's camera to face the direction the teleporter was thrown
  (`Controller.SetControlRotation` _returnvalue (`KismetMathLibrary.MakeRotator` _returnvalue_roll_2 _returnvalue_pitch_2 _returnvalue_yaw)))

(fn `UserConstructionScript`
  (`parent.UserConstructionScript`))