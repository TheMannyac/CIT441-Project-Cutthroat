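; Enemy child Blueprint that periodically fires bullets at the player pawn.
; BeginPlay caches the player pawn as Target and starts a looping timer for FireAtTarget.
; FireAtTarget spawns an EnemyBullet at SpawnPoint, rotated toward a valid Target, and plays an attenuated sound there.
; When the Target is destroyed, a delayed handler reacquires the player pawn, rebinds the destroy event and restarts the timer.
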(event `self.ReceiveBeginPlay`
  (`parent.ReceiveBeginPlay`)
  (bind _output_get (set `self.Target` (`GameplayStatics.GetPlayerPawn` 0) :!label _label))
  (add `self.OnDestroyed` _output_get (delegate `FindPlayerAgain`))
  (`KismetSystemLibrary.K2_SetTimer` null "FireAtTarget" 2.0 true))

(event `self.ReceiveTick`
  (params (DeltaSeconds :type "Float (single-precision)"))
  (`parent.ReceiveTick` DeltaSeconds))

(event `FindPlayerAgain` :!signature `self.OnDestroyed`
  (params (DestroyedActor :type "Actor Object Reference"))
  (`KismetSystemLibrary.Delay` 2.0)
  (goto _label))

(fn `FireAtTarget`
  (bind _target (`self.Target`))
  (bind _returnvalue (`SceneComponent.K2_GetComponentLocation` (`self.SpawnPoint`)))
  (`/Engine/EditorBlueprintResources/StandardMacros.IsValid` _target
    (:`Is Valid`
      (`|SpawnActorFromClass` "/Game/Blueprints/EnemyBullet.EnemyBullet_C" (`KismetMathLibrary.MakeTransform` _returnvalue (`KismetMathLibrary.MakeRotFromX` (- (`self.K2_GetActorLocation` _target) _returnvalue))) "Undefined" "OverrideRootScale" null null)
      (`GameplayStatics.PlaySoundAtLocation` "/Game/Audio/NewSoundCue.NewSoundCue" _returnvalue (struct) 1.0 1.0 0.0 "/Game/Audio/NewSoundAttenuation.NewSoundAttenuation" "/Game/Audio/NewSoundConcurrency.NewSoundConcurrency" null))))

(fn `UserConstructionScript`
  (`parent.UserConstructionScript`))