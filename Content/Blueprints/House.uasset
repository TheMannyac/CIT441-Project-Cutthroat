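; House is an interactable actor that can be highlighted and blown up.
; Indicate and UnIndicate toggle custom depth rendering on the static mesh, and CanInteract always returns true.
; Activate hides the house by scaling it to zero, without destroying the actor, and spawns an explosion emitter at its location.
; An older material-swap highlight remains as unconnected logic, though BeginPlay still caches the original materials for it.
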(event `self.ReceiveBeginPlay`
  (set `self.OriginalMaterial` (`MeshComponent.GetMaterials` (`self.StaticMesh`))))

(event `/Game/Blueprints/Interfaces/Interactable.Activate`
  (`self.SetActorScale3D` (0.0 0.0 0.0))
  (`GameplayStatics.SpawnEmitterAtLocation` "/Game/ImportedAssets/MundellsStarterContent/ParticleSystems/Explosion.Explosion" (`self.K2_GetActorLocation`)))

(event `/Game/Blueprints/Interfaces/Interactable.Indicate`
  (`PrimitiveComponent.SetRenderCustomDepth` (`self.StaticMesh`) true))

(event `/Game/Blueprints/Interfaces/Interactable.UnIndicate`
  (`PrimitiveComponent.SetRenderCustomDepth` (`self.StaticMesh`) false))

(fn `CanInteract`
  (returns (CanInteract :type Boolean))
  (return true))

(fn `UserConstructionScript`)