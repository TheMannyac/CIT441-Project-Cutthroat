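; ArrowSign is a level decor actor that endlessly swings back and forth on its roll axis around its starting rotation.
; A timeline, played at a rate set by Speed, drives a roll offset toward negative DegreesToRotate, using its track value as both the lerp's start and alpha.
; Each finish flips Reverse and calls ChangeDirection, alternating forward and reverse playback without using Tick.
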(event `self.ReceiveBeginPlay`
  (set `self.OriginalRotation` (`self.K2_GetActorRotation`))
  (`TimelineComponent.SetPlayRate` (`self.ArrowRotation`) (`self.Speed`))
  (if (`self.Reverse`) :!label _label
    (bind (_direction _newtrack_0) (`Timeline|ArrowRotation` :!via `PlayFromStart` :!label _label_2)
      (:`Update`
        (`self.K2_SetActorRotation` (`KismetMathLibrary.MakeRotator` (+ (`KismetMathLibrary.Lerp` _newtrack_0 (* (`self.DegreesToRotate`) -1.0) _newtrack_0) (.roll (`self.OriginalRotation`))) (.pitch (`self.OriginalRotation`)) (.yaw (`self.OriginalRotation`)))))
      (:`Finished`
        (set `self.Reverse` (not (`self.Reverse`)))
        (`self.Change direction`)))
    (else
      (goto _label_2 :!via `ReverseFromEnd`))))

(event `Change direction`
  (goto _label))

(fn `UserConstructionScript`)