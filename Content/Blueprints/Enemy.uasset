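; Enemy pawn that wanders the navmesh around its spawn point and has health shown on a widget health bar, destroying itself at zero HP.
; BeginPlay snaps it onto the navmesh, then a Wandering/Resting state machine picks random projected points, moves via SimpleMoveToLocation, faces its velocity and rests on arrival.
; It doubles as a teaching example, with unwired alternative rotation and movement nodes and a pure-node re-evaluation pitfall demo.
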(event `self.ReceiveBeginPlay`
  (bind (_projectedlocation _returnvalue) (`NavigationSystemV1.K2_ProjectPointToNavigation` (`self.K2_GetActorLocation`) null null (100.0 100.0 10000.0)))
  (set `self.HP` (`self.maxHP`))
  ;[1 1 1] Cheating to initialize hp bar widget.
  (`self.TakeDamage` 0.0)
  (bind _output_get (set `self.CapsuleBottomOffset` (`KismetMathLibrary.MakeVector` 0.0 0.0 (`CapsuleComponent.CapsuleHalfHeight` (`self.Capsule`)))))
  (if _returnvalue
    (`self.K2_SetActorLocation` (+ _output_get _projectedlocation))
    (else
      (`KismetSystemLibrary.PrintString` "Enemy BeginPlay Reposition Error")))
  (set `self.WanderCenter` (`self.K2_GetActorLocation`))
  (`self.StartWandering`))

(event `self.ReceiveTick`
  (params (DeltaSeconds :type "Float (single-precision)"))
  (switch `/Game/Blueprints/EnemyStates` (`self.CurrentState`)
    (:`NewEnumerator1`
      (`self.UpdateWandering`))))

(fn `ChangeState`
  (params (`New State` :type "/Game/Blueprints/EnemyStates Enum" :default "NewEnumerator0"))
  (if (not (`|EnumEquality` `New State` (`self.CurrentState`)))
    (`|ExecutionSequence`
      (:`then_0`
        ;[1 1 1] Turn off old state, like invalidate timers it was using.
        (switch `/Game/Blueprints/EnemyStates` (`self.CurrentState`)))
      (:`then_1`
        (set `self.CurrentState` (`local.New State`)))
      (:`then_2`
        ;[1 1 1] Start new state.
        (switch `/Game/Blueprints/EnemyStates` (`self.CurrentState`)
          (:`NewEnumerator2`
            (`KismetSystemLibrary.K2_SetTimer` null "StartWandering" 3.0)))))))

(fn `Rotate to Face Direction`
  (params (Direction :type "Vector Structure"))
  (locals (DirectionXY :type "Vector Structure" :default (0.0 0.0 0.0)))
  ;[1 1 1] Just different ways to rotate to face a certain direction.
  (set `local.DirectionXY` (`KismetMathLibrary.MakeVector` Direction_X Direction_Y))
  (`self.K2_SetActorRotation` (`KismetMathLibrary.MakeRotFromX` (`local.DirectionXY`))))

(fn `StartWandering`
  (locals (ProjectedLocation :type "Vector Structure") (ProjectResult :type Boolean) (RandPoint :type "Vector Structure" :default (0.0 0.0 0.0)))
  (bind (_returnvalue_x _returnvalue_y) (`KismetMathLibrary.BreakVector` (`KismetMathLibrary.RandomUnitVector`)))
  (bind _randpoint (`local.RandPoint`))
  (bind _output_get (set `local.RandPoint` (+ (* (`KismetMathLibrary.Normal` (`KismetMathLibrary.MakeVector` _returnvalue_x _returnvalue_y)) (`KismetMathLibrary.RandomFloatInRange` 0.0 (`self.WanderRadius`))) (select `bool` (`self.UseWanderCenter`) :`false` (`self.K2_GetActorLocation`) :`true` (`self.WanderCenter`)))))
  (bind (_projectedlocation _returnvalue) (`NavigationSystemV1.K2_ProjectPointToNavigation` _output_get null null (100.0 100.0 10000.0)))
  (set `local.ProjectedLocation` _projectedlocation)
  (bind _output_get_2 (set `local.ProjectResult` _returnvalue))
  (if _output_get_2
    (bind _output_get_3 (set `self.TargetPosition` (`local.ProjectedLocation`)))
    (bind _returnvalue_2 (+ _output_get_3 (`self.CapsuleBottomOffset`)))
    (`KismetSystemLibrary.DrawDebugArrow` _returnvalue_2 (+ _returnvalue_2 (0.0 0.0 -50.0)) 100.0 (struct :`G` 1.0 :`A` 1.0) 10.0 7.5)
    (`self.ChangeState` "NewEnumerator1")
    (`AIBlueprintHelperLibrary.SimpleMoveToLocation` (`AIBlueprintHelperLibrary.GetAIController` self) (`self.TargetPosition`))
    (else
      (`KismetSystemLibrary.DrawDebugArrow` _randpoint (+ _randpoint (0.0 0.0 -50.0)) 100.0 (struct :`R` 1.0 :`A` 1.0) 10.0 7.5)
      (`KismetSystemLibrary.PrintString` "Can't Get There")
      (`KismetSystemLibrary.K2_SetTimer` null "StartWandering" 0.5))))

(fn `TakeDamage`
  (params (Damage :type "Float (double-precision)"))
  (set `self.HP` (- (`self.HP`) Damage))
  (bind _ashealth_bar (cast `/Game/Widgets/HealthBar` (`WidgetComponent.GetUserWidgetObject` (`self.Widget`))))
  (`ProgressBar.SetPercent` (`/Game/Widgets/HealthBar.ProgressBar_0` _ashealth_bar) (/ (`self.HP`) (`self.maxHP`)))
  (if (<= (`self.HP`) 0.0)
    (`self.K2_DestroyActor`)))

(fn `UpdateTargetDirectionAndDistance`
  (set `self.DistanceToTarget` (- (`KismetMathLibrary.VSize` (- (+ (`self.TargetPosition`) (`self.CapsuleBottomOffset`)) (`self.K2_GetActorLocation`))) (`CapsuleComponent.GetScaledCapsuleRadius` (`self.Capsule`)))))

(fn `UpdateWandering`
  (bind _velocity (`MovementComponent.Velocity` (`self.FloatingPawnMovement`)))
  (`|ExecutionSequence`
    (:`then_0`
      ;[1 1 1] Calculate distance and direction to target and rotate to face it if we are actually moving.
      (`self.UpdateTargetDirectionAndDistance`)
      (if (> (`KismetMathLibrary.VSizeSquared` _velocity) 5.0)
        (`self.Rotate to Face Direction` _velocity)))
    (:`then_1`
      ;[1 1 1] Check if we've reached the target.
      (if (< (`self.DistanceToTarget`) (* (`MovementComponent.K2_GetModifiedMaxSpeed` (`self.FloatingPawnMovement`)) (`GameplayStatics.GetWorldDeltaSeconds`) 5.0))
        (`self.ChangeState` "NewEnumerator2")))))

(fn `UserConstructionScript`)

(fn `VisualizeVisualScriptingsBiggestPitfall`
  (locals (LocalRandomPoint :type "Vector Structure"))
  (bind (_returnvalue_x _returnvalue_y) (`KismetMathLibrary.BreakVector` (`KismetMathLibrary.RandomUnitVector`)))
  (bind _output_get (set `local.LocalRandomPoint` (* (`KismetMathLibrary.Normal` (`KismetMathLibrary.MakeVector` _returnvalue_x _returnvalue_y)) (`KismetMathLibrary.RandomFloatInRange` 0.0 (`self.WanderRadius`)))))
  (bind _returnvalue (+ _output_get (`self.K2_GetActorLocation`)))
  (bind _returnvalue_2 (+ _returnvalue (0.0 0.0 -50.0)))
  ;[1 1 1] What will this do?
  (`KismetSystemLibrary.DrawDebugArrow` _returnvalue _returnvalue_2 100.0 (struct :`R` 1.0 :`A` 1.0) 10.0 10.0)
  (`KismetSystemLibrary.DrawDebugArrow` _returnvalue _returnvalue_2 100.0 (struct :`G` 1.0 :`A` 1.0) 10.0 7.5)
  (`KismetSystemLibrary.DrawDebugArrow` _returnvalue _returnvalue_2 100.0 (struct :`B` 1.0 :`A` 1.0) 10.0 5.0))