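; Test game mode that runs a timed race course, player respawning and the level's music.
; BeginRace starts a Tick-driven stopwatch shown in a widget; FinishRace resolves a win, loss or forfeit against the best time.
; Event dispatchers broadcast race state, while delayed timelines cue win and loss audio and restore level music, though RaceLost also fires OnRaceWon.
; Player destruction triggers a delayed respawn at the spawn point and rebinds the death handler.
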(event `self.ReceiveTick`
  (params (DeltaSeconds :type "Float (single-precision)"))
  (bind _coursetimerwidget (`self.courseTimerWidget`))
  ;[0 1 0.6211] Tick
  (`|ExecutionSequence`
    (:`then_0`
      ;;[1 1 1] Increemnt Race Stopwatch
      (if (`self.isRacing`)
        (set `self.raceTimer` (+ (`self.raceTimer`) (`KismetMathLibrary.FromSeconds` (`GameplayStatics.GetWorldDeltaSeconds`))))
        (`/Engine/EditorBlueprintResources/StandardMacros.IsValid` _coursetimerwidget
          (:`Is Valid`
            (`/Game/Blueprints/UI/courseTimerWdget.Update Timer Text` _coursetimerwidget (`self.raceTimer`))))))))

(event `Respawn`
  ;[0 0.652 1] Begin Play
  ;;[1 1 1] Respwn System
  (bind _asbp_player (cast `/Game/Blueprints/Player/bp_player` (`GameplayStatics.GetPlayerCharacter` 0) :!label _label))
  (add `self.OnDestroyed` _asbp_player (delegate `onPlayerDeath`)))

(event `self.ReceiveBeginPlay`
  ;[0 0.652 1] Begin Play
  (bind _returnvalue (`GameplayStatics.CreatePlayer` (`self.PlayerInt`)))
  (`Controller.Possess` _returnvalue (`GameplayStatics.GetPlayerPawn` (`self.PlayerInt`)))
  (`|ExecutionSequence`
    (:`then_0`
      (goto _label))
    (:`then_1`
      ;;[1 1 1] Music
      (bind _returnvalue_2 (`GameplayStatics.CreateSound2D` null 1.0 1.0 0.0 null))
      (set `self.Music` _returnvalue_2)
      (`self.Set New Music Track` (`self.LevelMusic`))
      ;;[1 1 1] Setup Race Stuff
      (set `self.bestTime` (`KismetMathLibrary.MakeTimespan` 0 0 0 20)))))

(event `onPlayerDeath` :!signature `self.OnDestroyed`
  (params (DestroyedActor :type "Actor Object Reference"))
  ;[0 0.652 1] Begin Play
  ;;[1 1 1] Respwn System
  (`GameplayStatics.SpawnSound2D` "/Game/ImportedAssets/Audio/goofy-yell.goofy-yell" 1.0 1.0 0.0 null)
  (`KismetSystemLibrary.Delay` 2.0)
  (bind _returnvalue (`|SpawnActorFromClass` "/Game/Blueprints/Player/bp_player.bp_player_C" (`self.Spawn Point`) "Undefined" "OverrideRootScale" null 1000.0 7000.0 500.0 10 null))
  (`Controller.Possess` (`GameplayStatics.GetPlayerController` 0) _returnvalue)
  (`self.Respawn`))

(event `Race Won`
  ;[1 1 1] Race Outcome Events
  (`|ExecutionSequence`
    (:`then_0`
      (set `self.bestTime` (`self.raceTimer`))
      (`self.On Race Won`))
    (:`then_1`
      ;;[1 1 1] Cosmetic Affects
      (`KismetSystemLibrary.Delay` (`self.race Complete Delay`))
      (`Timeline|Lose Effect Timeline` :!via `PlayFromStart`
        (:`Announcer`
          (`GameplayStatics.PlaySound2D` "/Game/ImportedAssets/Audio/SmashBros/vc_narration_newrecord.vc_narration_newrecord" 1.0 1.0 0.0 null null))
        (:`crowd cheer`
          (`GameplayStatics.PlaySound2D` "/Game/ImportedAssets/Audio/TF2/TF2_winCrowd.TF2_winCrowd" 1.0 1.0 0.0 null null))
        (:`Restore level music`
          (`self.Set New Music Track` (`self.LevelMusic`)))))))

(event `Race Lost`
  ;[1 1 1] Race Outcome Events
  (`KismetSystemLibrary.Delay` (`self.race Complete Delay`))
  (`Timeline|Timeline_0` :!via `PlayFromStart`
    (:`Announcer`
      (`GameplayStatics.PlaySound2D` "/Game/ImportedAssets/Audio/SmashBros/vc_narration_failure.vc_narration_failure" 1.0 1.0 0.0 null null))
    (:`crowd cheer`
      (`GameplayStatics.PlaySound2D` "/Game/ImportedAssets/Audio/TF2/TF2_failCrowd.TF2_failCrowd" 1.0 1.0 0.0 null null))
    (:`Restore level music`
      (`self.Set New Music Track` (`self.LevelMusic`))
      (`self.On Race Won`))))

(event `Race Forfeited`
  ;[1 1 1] Race Outcome Events
  (`KismetSystemLibrary.Delay` 0.2)
  (`GameplayStatics.PlaySound2D` "/Game/ImportedAssets/Audio/SmashBros/vc_narration_failure.vc_narration_failure" 1.0 1.0 0.0 null null)
  (`self.On Race Forfeit`)
  (`self.raceReset`))

(fn `Begin Race`
  (if (not (`self.isRacing`))
    (`self.Create Course TImer Widget`)
    (set `self.isRacing` true)
    (set `self.raceTimer` (`KismetMathLibrary.MakeTimespan` 0))
    (`self.Set New Music Track` (`self.RaceMusic`))
    (`GameplayStatics.PlaySound2D` "/Game/ImportedAssets/Audio/SmashBros/vc_narration_go.vc_narration_go" 1.0 1.0 0.0 null null)
    (`KismetSystemLibrary.PrintString` "Race Start" true true (struct :`R` 1.0 :`G` 0.936244 :`A` 1.0))
    (`self.On Race Begin`)))

(fn `Create Course TImer Widget`
  (`/Engine/EditorBlueprintResources/StandardMacros.IsValid` (`self.courseTimerWidget`)
    (:`Is Not Valid`
      (bind _returnvalue (`|CreateWidget` "/Game/Blueprints/UI/courseTimerWdget.courseTimerWdget_C" (`GameplayStatics.GetPlayerController` 0)))
      (bind _output_get (set `self.courseTimerWidget` _returnvalue))
      (`UserWidget.AddToViewport` _output_get 0))))

(fn `Finish Race`
  (params (raceAborted :type Boolean))
  (locals (outcome :type "/Game/Blueprints/GameModes/SingleplayerRaceOutcomes Enum"))
  (`|ExecutionSequence`
    (:`then_0`
      ;[1 1 1] Cleanup race
      (set `self.isRacing` false)
      (`KismetSystemLibrary.PrintString` (`KismetStringLibrary.Concat_StrStr` "Race complete with a time of " (`KismetTextLibrary.Conv_TextToString` (`KismetTextLibrary.AsTimespan_Timespan` (`self.raceTimer`)))))
      (`self.Set New Music Track` (`self.LevelMusic`) false))
    (:`then_1`
      ;[1 1 1] Determine Race outcome
      (if (`local.raceAborted`)
        (`self.Race Forfeited`)
        (set `local.outcome` "NewEnumerator2")
        (else
          (`GameplayStatics.PlaySound2D` "/Game/ImportedAssets/Audio/SmashBros/vc_narration_timeup.vc_narration_timeup" 1.0 1.0 0.0 null null)
          (bind _output_get (set `self.timeDifference` (- (`self.bestTime`) (`self.raceTimer`))))
          (if (> _output_get (`KismetMathLibrary.MakeTimespan` 0))
            (`self.Race Won`)
            (set `local.outcome` "NewEnumerator0")
            (else
              (`self.Race Lost`)
              (set `local.outcome` "NewEnumerator1"))))))
    (:`then_2`
      ;[1 1 1] Tell eveyone the news
      (`self.On Race Complete` (`local.outcome`)))))

(fn `raceReset`
  (`self.Set New Music Track` (`self.LevelMusic`))
  (return))

(fn `Set New Music Track`
  (params (MusicTrack :type "SoundBase Object Reference") (playOnSet :type Boolean :default true) (startDelay :type "Float (double-precision)" :default 0.6))
  (locals (stop :type Boolean) (`start delay` :type "Float (double-precision)" :default -1.525989))
  (bind _music (`self.Music`))
  (bind _musictrack (`local.MusicTrack`))
  (`/Engine/EditorBlueprintResources/StandardMacros.IsValid` MusicTrack
    (:`Is Valid`
      (`/Engine/EditorBlueprintResources/StandardMacros.IsValid` (`self.Music`)
        (:`Is Valid`
          (`AudioComponent.Stop` _music)
          (`AudioComponent.SetSound` _music _musictrack))
        (:`Is Not Valid`
          (bind _returnvalue (`GameplayStatics.CreateSound2D` _musictrack 0.8 1.0 0.5 null))
          (set `self.Music` _returnvalue)))
      (if (`local.playOnSet`)
        (`AudioComponent.Play` _music 0.0))
      (return))))

(fn `UserConstructionScript`)