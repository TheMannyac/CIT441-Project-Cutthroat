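; Player controller that toggles a pause menu, created at BeginPlay, with the exit-game input.
; EnablePause shows the menu and cursor and disables pawn input, and DisablePause reverses this; the world keeps running, as the SetGamePaused node is disconnected.
; A separate NewFunction0, not called here, sums the Value of every Gem actor into MaxGems and writes it to the player HUD.
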(event `self.ReceiveBeginPlay`
  (bind _returnvalue (`|CreateWidget` "/Game/Widgets/PauseMenu.PauseMenu_C" self))
  (set `self.Pause Menu` _returnvalue))

(event `InputAction|inp_ExitGame`
  (params (Key :type "Key Structure"))
  (:`Pressed`
    (if (`Widget.IsInViewport` (`self.Pause Menu`))
      (`self.DisablePause`)
      (else
        (`self.EnablePause`)))))

(fn `DisablePause`
  (`Widget.RemoveFromParent` (`self.Pause Menu`))
  (set `self.bShowMouseCursor` false)
  (`self.EnableInput` (`GameplayStatics.GetPlayerPawn` 0) self)
  (`WidgetBlueprintLibrary.SetInputMode_GameOnly` self))

(fn `EnablePause`
  (`UserWidget.AddToViewport` (`self.Pause Menu`) 0)
  (set `self.bShowMouseCursor` true)
  (`self.DisableInput` (`self.K2_GetPawn`) self)
  (`WidgetBlueprintLibrary.SetInputMode_GameAndUIEx` self null))

(fn `NewFunction_0`
  ;[1 1 1] Figure out max gems amount
  (bind _outactors (`GameplayStatics.GetAllActorsOfClass` "/Game/Blueprints/Collectables/gem.gem_C"))
  (for _array_element _outactors
    (set `self.maxGems` (+ (`self.maxGems`) (`/Game/Blueprints/Collectables/gem.value` _array_element))))
  (`TextBlock.SetText` (`/Game/Blueprints/Player/playerHUD.MaxGemsText` (`self.Player hud`)) (`KismetTextLibrary.Conv_IntToText` (`self.maxGems`))))

(fn `UserConstructionScript`)