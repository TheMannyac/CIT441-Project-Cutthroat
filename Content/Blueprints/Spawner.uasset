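; Spawner actor that keeps spawning ClassToSpawn on a timer until MaxSpawns live instances exist.
; Each spawn's OnDestroyed lowers the count and restarts the timer if it is inactive, replenishing destroyed actors.
; Spawn points are random, either inside a box or on the edge of a horizontal circle, both sized by Diameter.
; The construction script scales and sets the SpawnIndicator mesh to preview the area.
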(event `self.ReceiveBeginPlay`
  (if (> (`self.MaxSpawns`) 0)
    (`KismetSystemLibrary.K2_SetTimer` null "SpawnEvent" (`self.TimeBetweenSpawns`))))

(event `SpawnEvent`
  (bind _spawned_actor (`self.SpawnAtRandomPoint`))
  (`/Engine/EditorBlueprintResources/StandardMacros.IncrementInt` (`self.CurrentSpawns`)
    (:`  `
      (add `self.OnDestroyed` _spawned_actor (delegate `SpawnDestroyed`))
      (if (not (== (`self.CurrentSpawns`) (`self.MaxSpawns`)))
        (bind _returnvalue (`KismetSystemLibrary.K2_SetTimer` null "SpawnEvent" (`self.TimeBetweenSpawns`) :!label _label))
        (set `self.SpawnTimer` _returnvalue)))))

(event `SpawnDestroyed` :!signature `self.OnDestroyed`
  (params (DestroyedActor :type "Actor Object Reference"))
  (`/Engine/EditorBlueprintResources/StandardMacros.DecrementInt` (`self.CurrentSpawns`)
    (:`  `
      (if (not (`KismetSystemLibrary.K2_IsTimerActiveHandle` (`self.SpawnTimer`)))
        (goto _label)))))

(fn `SpawnAtRandomPoint`
  (returns (`Spawned Actor` :type "Actor Object Reference"))
  (locals (RandomPosition :type "Vector Structure" :default (0.0 0.0 0.0)) (RandomUnitVec :type "Vector Structure" :default (0.0 0.0 0.0)))
  (bind (_returnvalue_x _returnvalue_y) (`KismetMathLibrary.BreakVector` (`KismetMathLibrary.RandomUnitVector`)))
  (bind (_returnvalue_x_2 _returnvalue_y_2) (`KismetMathLibrary.BreakVector` (`KismetMathLibrary.Conv_DoubleToVector` (/ (`self.Diameter`) 2.0))))
  (bind _returnvalue (`|SpawnActorFromClass` (`self.ClassToSpawn`) (`KismetMathLibrary.MakeTransform` (select `bool` (`self.UseBoxShape`) :`false` (+ (`self.K2_GetActorLocation`) (* (`KismetMathLibrary.Normal` (`KismetMathLibrary.MakeVector` _returnvalue_x _returnvalue_y)) (/ (`self.Diameter`) 2.0))) :`true` (`KismetMathLibrary.RandomPointInBoundingBox` (`self.K2_GetActorLocation`) (`KismetMathLibrary.MakeVector` _returnvalue_x_2 _returnvalue_y_2)))) "AlwaysSpawn" "OverrideRootScale" null null))
  (return _returnvalue))

(fn `UserConstructionScript`
  (bind _spawnindicator (`self.SpawnIndicator`))
  (`SceneComponent.SetWorldScale3D` (`self.SpawnIndicator`) (`KismetMathLibrary.Conv_DoubleToVector` (/ (`self.Diameter`) 100.0)))
  (if (`self.UseBoxShape`)
    (`StaticMeshComponent.SetStaticMesh` _spawnindicator null)
    (else
      (`StaticMeshComponent.SetStaticMesh` _spawnindicator null))))